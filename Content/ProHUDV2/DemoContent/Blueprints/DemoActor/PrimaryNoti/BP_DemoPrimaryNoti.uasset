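; Demo trigger actor for ProHUD V2 that shows a primary notification from its NotiInfo when a ThirdPersonCharacter overlaps its box.
; The notification is created through the HUD Manager.
; The construction script builds a dynamic material for the billboard, applying the notification's background icon texture and color plus an emissive power, then resizes the sprite element to Size.
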(event OnComponentBeginOverlap(Box)
  (params (OverlappedComponent :type Primitive%20Component%20Object%20Reference) (OtherActor :type Actor%20Object%20Reference) (OtherComp :type Primitive%20Component%20Object%20Reference) (OtherBodyIndex :type Integer) (bFromSweep :type Boolean) (SweepResult :type Hit%20Result%20Structure%20%28by%20ref%29))
  (Utilities|Casting|CastToThirdPersonCharacter OtherActor)
  (Default|CreatePrimaryNotification (CallFunction|GetHUDManager) (Variables|Default|GetNotiInfo)))

(event Custom|UpdateActor
  (bind _notiinfo (Variables|Default|GetNotiInfo))
  (bind _backgroundiconinfo (Utilities|Struct|BreakS_PrimaryNotiInfo _notiinfo))
  (bind (_icontexture _transform _iconcolor) (Utilities|Struct|BreakS_IconInfo2 _backgroundiconinfo))
  (bind (_r _g _b) (Utilities|Struct|BreakLinearColor _iconcolor))
  (|CreateDynamicMaterialforBillboard22)
  (|SetMaterialTexture22 (.AsTexture (Utilities|Casting|CastToTexture _icontexture)))
  (|SetMaterialColor22 (Math|Color|MakeColor _r _g _b))
  (|SetMaterialEmissive22 (Variables|Default|GetEmissivePower))
  (|FinishMaterial22))

(fn ConstructionScript
  (CallFunction|UpdateActor))