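; Playing card actor whose front and back materials are picked from arrays by set, suit, rank and back style, in the construction script or via SetCardValue.
; Rotate and Unrotate play a timeline forward or in reverse to flip and shift the card in one of four directions, with sound.
; While the player can take a turn, hovering an unflipped card raises it, outlines it via custom depth, and prints debug info.
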(event OnBeginCursorOver(PlayingCard)
  (params (TouchedComponent :type Primitive%20Component%20Object%20Reference))
  (bind _returnvalue (Game|GetPlayerController 0))
  (bind _playingcard (Variables|Default|GetPlayingCard))
  (bind (_worldlocation _worlddirection) (Game|Player|ConvertMouseLocationToWorldSpace _returnvalue))
  (bind _output_get (Variables|Default|SetTouched%20Component TouchedComponent))
  (bind _aschar_rof (Utilities|Casting|CastToCHAR_ROF (Game|GetPlayerCharacter 0)))
  (if (not (Variables|Default|GetIsFlipped?))
    (if (Variables|/Game/Ultimate_Ring_Of_Fire/Character/CHAR_ROF.CHAR_ROF_C|GetCanTakeTurn? _aschar_rof)
      (Development|PrintString (Utilities|String|ToString(Float) (+ (Variables|/Game/Ultimate_Ring_Of_Fire/Character/CHAR_ROF.CHAR_ROF_C|GetZ%20Order _aschar_rof) 1.0)))
      (Transformation|SetWorldLocation _output_get (Math|Vector|MakeVector (.x (Transformation|GetWorldLocation _output_get)) (.y (Transformation|GetWorldLocation _output_get)) (+ (Variables|/Game/Ultimate_Ring_Of_Fire/Character/CHAR_ROF.CHAR_ROF_C|GetZ%20Order _aschar_rof) 1.0)) false false)
      (Rendering|SetRenderCustomDepth _playingcard true)
      (Rendering|SetCustomDepthStencilValue _playingcard 2)
      (bind _outhit (Collision|LineTraceByChannel _worldlocation (+ _worldlocation (* _worlddirection 3e+04)) "TraceTypeQuery1" false 0 "None" false))
      (bind _asbp_playing_card (Utilities|Casting|CastToBP_Playing_Card (.HitActor (Collision|BreakHitResult _outhit))))
      (Development|PrintString (Utilities|String|Append (Utilities|String|EnumtoString (Variables|BP_Playing_Card_C|GetCardRank _asbp_playing_card)) " / " (Utilities|String|EnumtoString (Variables|BP_Playing_Card_C|GetCardSuits _asbp_playing_card)))))))

(event OnEndCursorOver(PlayingCard)
  (params (TouchedComponent :type Primitive%20Component%20Object%20Reference))
  (bind _playingcard (Variables|Default|GetPlayingCard))
  (Variables|Default|SetTouched%20Component TouchedComponent)
  (bind _aschar_rof (Utilities|Casting|CastToCHAR_ROF (Game|GetPlayerCharacter 0)))
  (if (not (Variables|Default|GetIsFlipped?))
    (if (Variables|/Game/Ultimate_Ring_Of_Fire/Character/CHAR_ROF.CHAR_ROF_C|GetCanTakeTurn? _aschar_rof)
      (Transformation|SetWorldLocation (Variables|Default|GetTouched%20Component) (Math|Vector|MakeVector (.x (Transformation|GetWorldLocation (Variables|Default|GetTouched%20Component))) (.y (Transformation|GetWorldLocation (Variables|Default|GetTouched%20Component))) (Variables|Default|GetDefaultCardLocation)) false false)
      (Rendering|SetRenderCustomDepth _playingcard false)
      (Rendering|SetCustomDepthStencilValue _playingcard 0)
      (Development|PrintString (Utilities|String|ToString(Float) (Variables|Default|GetDefaultCardLocation))))))

(event Custom|Rotate
  (bind _cardrotation (Variables|Default|GetCardRotation))
  ;[1 1 1] Rotate/Unrotate Card
  (if (Variables|Default|GetcanRotate)
    (Variables|Default|SetcanRotate false)
    (if (Utilities|Enum|Equal(Enum) _cardrotation "NewEnumerator0")
      (Variables|Default|SetRotationDir -1.0)
      (Variables|Default|SetStartPosition (Transformation|GetActorLocation))
      (Variables|Default|SetEndPosition (+ (Variables|Default|GetStartPosition) "0,-50.000000,50.000000"))
      (Variables|Default|SetStartRotation (Math|Rotator|MakeRotator 359.0 0.0 0.0))
      (Variables|Default|SetEndRotation (Math|Rotator|MakeRotator 179.0 0.0 0.0))
      ;;[1 1 1] Card Rotates - Sound FX
      (Utilities|FlowControl|Sequence :!label _label
        (:then_0
          (Utilities|FlowControl|Delay 0.05)
          (bind (_direction _newtrack_0 _newtrack_1) (Timeline|Timeline_0 PlayFromStart)
            (:Update
              (Transformation|SetActorRelativeTransform (Math|Transform|MakeTransform (Math|Vector|Lerp(Vector) (Variables|Default|GetStartPosition) (Variables|Default|GetEndPosition) _newtrack_1) (Math|Rotator|Lerp(Rotator) (Variables|Default|GetStartRotation) (Variables|Default|GetEndRotation) (* _newtrack_0 (Variables|Default|GetRotationDir)))) false false))
            (:Finished
              (Variables|Default|SetcanRotate true))))
        (:then_1
          (Audio|PlaySoundatLocation 0 "0, 0, 0" "0, 0, 0" 1.0 1.0 0.0 0 0 0 0)))
      (elif (Utilities|Enum|Equal(Enum) _cardrotation "NewEnumerator1")
        (Variables|Default|SetRotationDir 1.0)
        (Variables|Default|SetStartPosition (Transformation|GetActorLocation))
        (Variables|Default|SetEndPosition (+ (Variables|Default|GetStartPosition) "0,50.000000,50.000000"))
        (Variables|Default|SetStartRotation (Math|Rotator|MakeRotator 359.0 0.0 0.0))
        (Variables|Default|SetEndRotation (Math|Rotator|MakeRotator 179.0 0.0 0.0))
        (goto _label)
        (elif (Utilities|Enum|Equal(Enum) _cardrotation "NewEnumerator2")
          (Variables|Default|SetRotationDir -1.0)
          (Variables|Default|SetStartPosition (Transformation|GetActorLocation))
          (Variables|Default|SetEndPosition (+ (Variables|Default|GetStartPosition) "50.000000,0.000000,50.000000"))
          (Variables|Default|SetStartRotation (Math|Rotator|MakeRotator 0.0 359.0 0.0))
          (Variables|Default|SetEndRotation (Math|Rotator|MakeRotator 0.0 179.0 0.0))
          (goto _label)
          (elif (Utilities|Enum|Equal(Enum) _cardrotation "NewEnumerator3")
            (Variables|Default|SetRotationDir -1.0)
            (Variables|Default|SetStartPosition (Transformation|GetActorLocation))
            (Variables|Default|SetEndPosition (+ (Variables|Default|GetStartPosition) "-50.000000,0.000000,50.000000"))
            (Variables|Default|SetStartRotation (Math|Rotator|MakeRotator 0.0 0.0 0.0))
            (Variables|Default|SetEndRotation (Math|Rotator|MakeRotator 0.0 179.0 0.0))
            (goto _label)))))))

(event Custom|Unrotate
  (bind _cardrotation (Variables|Default|GetCardRotation))
  ;[1 1 1] Rotate/Unrotate Card
  (if (Variables|Default|GetcanRotate)
    (Variables|Default|SetcanRotate false)
    (if (Utilities|Enum|Equal(Enum) _cardrotation "NewEnumerator0")
      (Variables|Default|SetRotationDir 1.0)
      (Variables|Default|SetEndPosition (+ (Variables|Default|GetStartPosition) "0,-50.000000,50.000000"))
      (Variables|Default|SetStartPosition (Variables|Default|GetStartPosition))
      (Variables|Default|SetStartRotation (Math|Rotator|MakeRotator 359.0 0.0 0.0))
      (Variables|Default|SetEndRotation (Math|Rotator|MakeRotator 179.0 0.0 0.0))
      ;;[1 1 1] Card Rotates - Sound FX
      (Utilities|FlowControl|Sequence :!label _label
        (:then_0
          (Audio|PlaySoundatLocation 0 "0, 0, 0" "0, 0, 0" 1.0 1.0 0.0 0 0 0 0))
        (:then_1
          (Utilities|FlowControl|Delay 0.05)
          (bind (_direction _newtrack_0 _newtrack_1) (Timeline|Timeline_0 ReverseFromEnd)
            (:Update
              (Transformation|SetActorRelativeTransform (Math|Transform|MakeTransform (Math|Vector|Lerp(Vector) (Variables|Default|GetStartPosition) (Variables|Default|GetEndPosition) _newtrack_1) (Math|Rotator|Lerp(Rotator) (Variables|Default|GetStartRotation) (Variables|Default|GetEndRotation) (* _newtrack_0 (Variables|Default|GetRotationDir)))) false false))
            (:Finished
              (Variables|Default|SetcanRotate true)))))
      (elif (Utilities|Enum|Equal(Enum) _cardrotation "NewEnumerator1")
        (Variables|Default|SetRotationDir -1.0)
        (Variables|Default|SetEndPosition (+ (Variables|Default|GetStartPosition) "0,50.000000,50.000000"))
        (Variables|Default|SetStartPosition (Variables|Default|GetStartPosition))
        (Variables|Default|SetStartRotation (Math|Rotator|MakeRotator 359.0 0.0 0.0))
        (Variables|Default|SetEndRotation (Math|Rotator|MakeRotator 179.0 0.0 0.0))
        (goto _label)
        (elif (Utilities|Enum|Equal(Enum) _cardrotation "NewEnumerator2")
          (Variables|Default|SetRotationDir 1.0)
          (Variables|Default|SetEndPosition (+ (Variables|Default|GetStartPosition) "50.000000,0.000000,50.000000"))
          (Variables|Default|SetStartPosition (Variables|Default|GetStartPosition))
          (Variables|Default|SetStartRotation (Math|Rotator|MakeRotator 0.0 359.0 0.0))
          (Variables|Default|SetEndRotation (Math|Rotator|MakeRotator 0.0 179.0 0.0))
          (goto _label)
          (elif (Utilities|Enum|Equal(Enum) _cardrotation "NewEnumerator3")
            (Variables|Default|SetRotationDir 1.0)
            (Variables|Default|SetEndPosition (+ (Variables|Default|GetStartPosition) "-50.000000,0.000000,50.000000"))
            (Variables|Default|SetStartPosition (Variables|Default|GetStartPosition))
            (Variables|Default|SetStartRotation (Math|Rotator|MakeRotator 0.0 0.0 0.0))
            (Variables|Default|SetEndRotation (Math|Rotator|MakeRotator 0.0 179.0 0.0))
            (goto _label)))))))

(event EventBeginPlay
  (if (Variables|Default|GetAutoRotates)
    (CallFunction|SetCardValue "NewEnumerator17" "NewEnumerator0" "NewEnumerator1" "NewEnumerator45")
    (CallFunction|Rotate)))

(fn ConstructionScript
  (bind _cardsets (Variables|Default|GetCardSets))
  (bind _cardsuits (Variables|Default|GetCardSuits))
  (bind _cardrank (Variables|Default|GetCardRank))
  (bind _cards (Variables|Default|GetCards))
  (bind _deckback (Variables|Default|GetDeckBack))
  (bind _cardbacks (Variables|Default|GetCardBacks))
  (bind _returnvalue (Utilities|Select :Index _cardsets :NewEnumerator0 0 :NewEnumerator1 52 :NewEnumerator2 104 :NewEnumerator17 156))
  (bind _returnvalue_2 (Utilities|Select :Index _cardsuits :NewEnumerator0 0 :NewEnumerator1 13 :NewEnumerator2 26 :NewEnumerator3 39))
  (bind _returnvalue_3 (Utilities|Select :Index _cardrank :NewEnumerator1 0 :NewEnumerator2 1 :NewEnumerator3 2 :NewEnumerator4 3 :NewEnumerator5 4 :NewEnumerator6 5 :NewEnumerator7 6 :NewEnumerator8 7 :NewEnumerator9 8 :NewEnumerator10 9 :NewEnumerator11 10 :NewEnumerator12 11 :NewEnumerator13 12))
  (bind _returnvalue_4 (Utilities|Select :Index _deckback :NewEnumerator1 0 :NewEnumerator2 1 :NewEnumerator3 2 :NewEnumerator4 3 :NewEnumerator5 4 :NewEnumerator6 5 :NewEnumerator7 6 :NewEnumerator8 7 :NewEnumerator9 8 :NewEnumerator10 9 :NewEnumerator11 10 :NewEnumerator12 11 :NewEnumerator13 12 :NewEnumerator14 13 :NewEnumerator15 14 :NewEnumerator16 15 :NewEnumerator17 16 :NewEnumerator18 17 :NewEnumerator19 18 :NewEnumerator20 19 :NewEnumerator21 20 :NewEnumerator22 21 :NewEnumerator23 22 :NewEnumerator24 23 :NewEnumerator25 24 :NewEnumerator37 25 :NewEnumerator38 26 :NewEnumerator39 27 :NewEnumerator40 28 :NewEnumerator41 29 :NewEnumerator42 30 :NewEnumerator43 31 :NewEnumerator44 32 :NewEnumerator45 33 :NewEnumerator46 34 :NewEnumerator47 35 :NewEnumerator48 36))
  (bind _returnvalue_5 (+ _returnvalue _returnvalue_2 _returnvalue_3))
  (bind _output (Utilities|Array|Get(acopy) _cardbacks _returnvalue_4))
  (bind _output_2 (Utilities|Array|Get(acopy) _cards _returnvalue_5))
  (if (Variables|Default|GetAdvanced%20Settings)
    (Rendering|Material|SetMaterial (Variables|Default|GetPlayingCard) 0 _output_2)
    (Variables|Default|SetCardFront _output_2)
    (Rendering|Material|SetMaterial (Variables|Default|GetPlayingCard) 1 _output)
    (Variables|Default|SetCardBack _output)
    (else
      (Rendering|Material|SetMaterial (Variables|Default|GetPlayingCard) 0 (Variables|Default|GetCardFront))
      (Rendering|Material|SetMaterial (Variables|Default|GetPlayingCard) 1 (Variables|Default|GetCardBack)))))

(fn SetCardValue
  (params (CardSet :type E_CardSets%20Enum :default "NewEnumerator0") (CardSuit :type E_CardSuits%20Enum :default "NewEnumerator0") (CardRank :type E_CardRanks%20Enum :default "NewEnumerator1") (NewParam :type E_DeckBacks%20Enum :default "NewEnumerator1"))
  (bind _returnvalue (Utilities|Select :Index CardSet :NewEnumerator0 0 :NewEnumerator1 52 :NewEnumerator2 104 :NewEnumerator17 156))
  (bind _returnvalue_2 (Utilities|Select :Index CardSuit :NewEnumerator0 0 :NewEnumerator1 13 :NewEnumerator2 26 :NewEnumerator3 39))
  (bind _returnvalue_3 (Utilities|Select :Index CardRank :NewEnumerator1 0 :NewEnumerator2 1 :NewEnumerator3 2 :NewEnumerator4 3 :NewEnumerator5 4 :NewEnumerator6 5 :NewEnumerator7 6 :NewEnumerator8 7 :NewEnumerator9 8 :NewEnumerator10 9 :NewEnumerator11 10 :NewEnumerator12 11 :NewEnumerator13 12))
  (bind _returnvalue_4 (Utilities|Select :Index NewParam :NewEnumerator1 0 :NewEnumerator2 1 :NewEnumerator3 2 :NewEnumerator4 3 :NewEnumerator5 4 :NewEnumerator6 5 :NewEnumerator7 6 :NewEnumerator8 7 :NewEnumerator9 8 :NewEnumerator10 9 :NewEnumerator11 10 :NewEnumerator12 11 :NewEnumerator13 12 :NewEnumerator14 13 :NewEnumerator15 14 :NewEnumerator16 15 :NewEnumerator17 16 :NewEnumerator18 17 :NewEnumerator19 18 :NewEnumerator20 19 :NewEnumerator21 20 :NewEnumerator22 21 :NewEnumerator23 22 :NewEnumerator24 23 :NewEnumerator25 24 :NewEnumerator37 25 :NewEnumerator38 26 :NewEnumerator39 27 :NewEnumerator40 28 :NewEnumerator41 29 :NewEnumerator42 30 :NewEnumerator43 31 :NewEnumerator44 32 :NewEnumerator45 33 :NewEnumerator46 34 :NewEnumerator47 35 :NewEnumerator48 36))
  (bind _cards (Variables|Default|GetCards))
  (bind _cardbacks (Variables|Default|GetCardBacks))
  (bind _returnvalue_5 (+ _returnvalue _returnvalue_2 _returnvalue_3))
  (bind _output (Utilities|Array|Get(acopy) _cardbacks _returnvalue_4))
  (bind _output_2 (Utilities|Array|Get(acopy) _cards _returnvalue_5))
  (Rendering|Material|SetMaterial (Variables|Default|GetPlayingCard) 0 _output_2)
  (Variables|Default|SetCardFront _output_2)
  (Rendering|Material|SetMaterial (Variables|Default|GetPlayingCard) 1 _output)
  (Variables|Default|SetCardBack _output)
  (return))