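; BP_Dice is a configurable physics die that rolls on BeginPlay or click and broadcasts when a roll starts and stops.
; Roll moves the die to an Arrow actor by Magnet timeline or teleport, then launches it with randomized direction, velocity and spin.
; Tick watches for near-zero speed, then reports the highest mesh socket's name as the result.
; Hard hits can play impact sounds, and collisions while moving can optionally signal a new roll.
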(event OnClicked(Dice)
  (params (TouchedComponent :type Primitive%20Component%20Object%20Reference) (ButtonPressed :type Key%20Structure :default "None"))
  ;[1 1 1] Roll on Mouse click
  (CallFunction|Roll))

(event OnComponentHit(Dice)
  (params (HitComponent :type Primitive%20Component%20Object%20Reference) (OtherActor :type Actor%20Object%20Reference) (OtherComp :type Primitive%20Component%20Object%20Reference) (NormalImpulse :type Vector :default "0, 0, 0") (Hit :type Hit%20Result%20Structure%20%28by%20ref%29))
  (bind _returnvalue (Math|Vector|VectorLength NormalImpulse))
  (Utilities|FlowControl|Sequence
    (:then_0
      ;[1 1 1] When Dice is hitted by other object and have significant velocity, Start Roll will be called
      (if (Variables|Default|GetStart%20Roll%20from%20other%20objects)
        (bind _returnvalue_2 (Physics|GetPhysicsLinearVelocity (Variables|Default|GetDice) "None"))
        (if (> (Math|Vector|VectorLength _returnvalue_2) 5.0)
          (Variables|Default|SetIsMoving true)
          (Default|CallStartRoll))))
    (:then_1
      ;[1 1 1] Sound
      (if (and (> _returnvalue 5e+03) (Variables|Default|GetHit%20Sound))
        (Audio|PlaySound2D (Utilities|Select :Index (Math|Random|RandomInteger 2) :Option%200 "/Game/Dices/Sounds/Dice_2.Dice_2" :Option%201 "/Game/Dices/Sounds/Dice_3.Dice_3" :Option%202 "/Game/Dices/Sounds/Dice_1.Dice_1") (* _returnvalue 0.0001 (Variables|Default|GetVolume)) 1.0 0.0 0 0)))))

(event Custom|Roll
  (bind _returnvalue (Math|Random|RandomUnitVector))
  (bind _arrow (Variables|Default|GetArrow))
  (bind _dice (Variables|Default|GetDice))
  (bind _random_velocity__ (Variables|/Game/Dices/Blueprints/BP_StartingArrow.BP_StartingArrow_C|GetRandom%20Velocity%20%25 _arrow))
  (bind _random_direction (Variables|/Game/Dices/Blueprints/BP_StartingArrow.BP_StartingArrow_C|GetRandom%20Direction _arrow))
  (bind _returnvalue_2 (* 1.6e+02 _random_direction))
  (bind _returnvalue_3 (* _returnvalue _returnvalue_2))
  (bind (_x _y _z) (Math|Vector|BreakVector _returnvalue_3))
  (Utilities|IsValid (Variables|Default|GetArrow)
    (:Is%20Valid
      (if (Variables|Magnet|GetMagnet%20to%20Arrow)
        ;[1 1 1] Magnet to Arrow
        (Variables|Magnet|SetIs%20magneting%20now true)
        (bind _output_get (Variables|Magnet|SetMagnet%20starting%20Dice%20location (Transformation|GetWorldLocation (Variables|Default|GetDice))))
        (bind _magnet (Timeline|Magnet PlayFromStart)
          (:Update
            (Transformation|SetWorldLocation (Variables|Default|GetDice) (Math|Vector|Lerp(Vector) _output_get (Transformation|GetWorldLocation (Variables|/Game/Dices/Blueprints/BP_StartingArrow.BP_StartingArrow_C|GetArrow (Variables|Default|GetArrow))) _magnet) false false))
          (:Finished
            (Variables|Magnet|SetIs%20magneting%20now false)
            ;[1 1 1] Launch Dice from Arrow
            (Transformation|SetWorldRotation _dice (Math|Random|RandomRotator false) false false :!label _label)
            (Physics|SetPhysicsLinearVelocity _dice (* (Math|Vector|RotateVector (Math|Vector|GetForwardVector (Variables|/Script/Engine.Actor|GetRootComponent _arrow)) (Math|Rotator|MakeRotator _x _y _z)) (* (Variables|/Game/Dices/Blueprints/BP_StartingArrow.BP_StartingArrow_C|GetStarting%20Velocity%20%28cm/s%29 _arrow) (+ (Math|Random|RandomFloatinRange (/ _random_velocity__ -1e+02) (/ _random_velocity__ 1e+02)) 1.0))) false "None")
            (Class|PrimitiveComponent|SetPhysicsAngularVelocityinDegrees _dice (* (Math|Random|RandomUnitVector) (Math|Random|RandomFloatinRange 0.0 5e+01)) false "None")
            (Default|CallStartRoll)
            (Utilities|FlowControl|Delay 0.1)
            (Variables|Default|SetIsMoving true)))
        (else
          ;[1 1 1] Teleport to Arrow
          (Transformation|SetWorldLocation (Variables|Default|GetDice) (Transformation|GetWorldLocation (Variables|/Script/Engine.Actor|GetRootComponent (Variables|Default|GetArrow))) false true)
          (goto _label))))
    (:Is%20Not%20Valid
      (Development|PrintString "No Arrow selected"))))

(event EventBeginPlay
  ;[1 1 1] Roll on BeginPlay
  (if (Variables|Default|GetRoll%20on%20BeginPlay)
    (CallFunction|Roll)))

(event EventTick
  (params (DeltaSeconds :type Float%20%28single-precision%29))
  (bind _dice (Variables|Default|GetDice))
  (bind _socket_z_height (Variables|Default|GetSocket%20Z%20height))
  (bind _returnvalue (Transformation|GetAllSocketNames _dice))
  ;[1 1 1] Whether dice speed should be watched
  (if (not (Variables|Magnet|GetIs%20magneting%20now))
    (if (Variables|Default|GetIsMoving)
      ;[1 1 1] Check if Dice stopped
      (bind _returnvalue_2 (Physics|GetPhysicsLinearVelocity (Variables|Default|GetDice) "None"))
      (if (< (Math|Vector|VectorLength _returnvalue_2) 0.5)
        (Utilities|FlowControl|Delay 0.2)
        (Variables|Default|SetIsMoving false)
        ;[1 1 1] Determine Roll Result
        (Utilities|Array|Clear (Variables|Default|GetSocket%20Z%20height))
        (for _array_element _returnvalue
          (Utilities|Array|Add _socket_z_height (.z (Transformation|GetSocketLocation _dice _array_element))))
        (bind _output_get (Variables|Default|SetRoll%20Result (Utilities|Array|Get(acopy) _returnvalue (.IndexOfMaxValue (Math|Float|MaxOfFloatArray _socket_z_height)))))
        (Default|CallStopRoll _output_get)))))

(fn ConstructionScript
  (bind _dice (Variables|Default|GetDice))
  (bind _size__cm_ (Variables|Default|GetSize%20%28cm%29))
  (bind _returnvalue (/ _size__cm_ 5.0))
  (Components|StaticMesh|SetStaticMesh _dice (Variables|Appearance|GetDice%20Mesh))
  (Rendering|Material|SetMaterial _dice 0 (Variables|Appearance|GetMaterial%201))
  (if (> (Rendering|Material|GetNumMaterials _dice) 1)
    (Rendering|Material|SetMaterial _dice 1 (Variables|Appearance|GetMaterial%202)))
  (Transformation|SetWorldScale3D _dice (Math|Vector|MakeVector _returnvalue _returnvalue _returnvalue))
  (Components|Timeline|SetPlayRate (Variables|Default|GetMagnet) (Variables|Magnet|GetMagnet%20speed)))